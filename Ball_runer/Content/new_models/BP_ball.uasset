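; BP_ball is a player-controlled rolling ball with health, moved by applying torque from two input axes.
; Overlaps with healing points and damage spikes change health; passing 40 triggers a one-time scaling, while dropping below zero fades out and reloads the level.
; Camera-activation overlaps alternate between two cameras and toggle ISChange, which flips the sign of X torque.
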(event EventBeginPlay
  ;[1 1 1] fade kamery na start gry
  (CameraFades|StartCameraFade (Game|GetPlayerCameraManager 0) 1.0 0.0 1.0 "(R=0.045770,G=0.037477,B=0.095833,A=1.000000)" false false)
  (Variables|Default|SetIS%20change true))

(event Collision|EventActorBeginOverlap
  (params (OtherActor :type Actor%20Object%20Reference))
  ;[1 1 1] heal i DMG
  (Utilities|FlowControl|Sequence
    (:then_0
      (Utilities|Casting|CastToHealing_point OtherActor)
      (CallFunction|Heal))
    (:then_1
      (Utilities|Casting|CastToDamage_spices OtherActor)
      (CallFunction|GedDmg)
      (if (< (Variables|Default|GetHealth) 0.0)
        (CameraFades|StartCameraFade :self (Game|GetPlayerCameraManager 0) :ToAlpha 1.0 :Duration 1.0)
        (bind _returnvalue (Game|GetCurrentLevelName true))
        (Utilities|FlowControl|Delay 1.0)
        (Game|OpenLevel(byName) (Utilities|String|StringToName _returnvalue))))
    (:then_2
      ;[1 1 1] zmiana kamery
      (Utilities|Casting|CastToAktywacja_kamery OtherActor)
      (Utilities|FlowControl|FlipFlop
        (:A
          (Components|Activation|SetActive (Variables|Default|GetCamera) false false)
          (Components|Activation|SetActive (Variables|Default|GetCamera1) true false)
          (Variables|Default|SetIS%20change false))
        (:B
          (Components|Activation|SetActive (Variables|Default|GetCamera) true false)
          (Components|Activation|SetActive (Variables|Default|GetCamera1) false false)
          (Variables|Default|SetIS%20change true))))))

(event Input|AxisEvents|InputAxisMoveForward/backward
  (params (AxisValue :type Float%20%28single-precision%29))
  (bind _predkosc_obrotowa (Variables|Default|Getpredkosc%20obrotowa))
  ;[1 1 1] Krecenie się (siła)
  (if (Variables|Default|GetIS%20change)
    (Class|PrimitiveComponent|AddTorqueinRadians (Variables|Default|Getball) (Math|Vector|MakeVector (* (stale Input|AxisEvents|InputAxisMoveleft/right AxisValue) _predkosc_obrotowa) (* AxisValue _predkosc_obrotowa) 0.0) "None" true)
    (else
      (Class|PrimitiveComponent|AddTorqueinRadians (Variables|Default|Getball) (Math|Vector|MakeVector (* (* AxisValue _predkosc_obrotowa) -1.0) (* (stale Input|AxisEvents|InputAxisMoveleft/right AxisValue) _predkosc_obrotowa) 0.0) "None" true))))

(event Input|AxisEvents|InputAxisMoveleft/right
  (params (AxisValue :type Float%20%28single-precision%29))
  (bind _predkosc_obrotowa (Variables|Default|Getpredkosc%20obrotowa))
  ;[1 1 1] Krecenie się (siła)
  (if (Variables|Default|GetIS%20change)
    (Class|PrimitiveComponent|AddTorqueinRadians (Variables|Default|Getball) (Math|Vector|MakeVector (* AxisValue _predkosc_obrotowa) (* (stale Input|AxisEvents|InputAxisMoveForward/backward AxisValue) _predkosc_obrotowa) 0.0) "None" true)
    (else
      (Class|PrimitiveComponent|AddTorqueinRadians (Variables|Default|Getball) (Math|Vector|MakeVector (* (* (stale Input|AxisEvents|InputAxisMoveForward/backward AxisValue) _predkosc_obrotowa) -1.0) (* AxisValue _predkosc_obrotowa) 0.0) "None" true))))

(fn ConstructionScript)

(fn GedDmg
  (Variables|Default|SetHealth (- (Variables|Default|GetHealth) 8.0))
  (Effects|SpawnEmitteratLocation "/Game/AdvancedMagicFX12/particles/P_ky_hit_shine.P_ky_hit_shine" (Transformation|GetActorLocation))
  (Development|PrintString "-8" true true "(R=1.000000,G=0.095909,B=0.000000,A=1.000000)"))

(fn Heal
  (bind _set_health (Utilities|Healing (Variables|Default|GetHealth))
    (:Out
      (Variables|Default|SetHealth _set_health)
      (Development|PrintString "+10" true true "(R=0.106973,G=1.000000,B=0.000000,A=1.000000)")
      (if (> (Variables|Default|GetHealth) 4e+01)
        (if (not (Variables|Default|Getis%20scaled))
          (Utilities|Scaleing self
            (:out
              (Variables|Default|Setis%20scaled true))))))))